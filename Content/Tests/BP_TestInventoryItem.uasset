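; Test inventory item Blueprint that holds inventory data and a color.
; SetInventoryData stores both values, then calls Init, which is not defined in this graph.
; CalculateColor returns the stored Color unchanged.
; The default BeginPlay, overlap and Tick events are disabled, and the construction script only calls its parent.
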(event Custom|SetInventoryData
  (params (InventoryData :type Inventory%20Data%20Structure) (Color :type Linear%20Color%20Structure))
  (Variables|Default|SetInventoryData InventoryData)
  (Variables|Default|SetColor Color)
  (CallFunction|Init))

(event EventBeginPlay
  (|CallParentFunction) ; This node is disabled and will not be called.\nDrag off pins to build functionality.
)

(event Collision|EventActorBeginOverlap
  (params (OtherActor :type Actor%20Object%20Reference))
  (|CallParentFunction OtherActor) ; This node is disabled and will not be called.\nDrag off pins to build functionality.
)

(event EventTick
  (params (DeltaSeconds :type Float%20%28single-precision%29))
  (|CallParentFunction DeltaSeconds) ; This node is disabled and will not be called.\nDrag off pins to build functionality.
)

(fn ConstructionScript
  (|CallParentFunction))

(fn CalculateColor
  (return (Variables|Default|GetColor)))