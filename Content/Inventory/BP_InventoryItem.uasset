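; BP_InventoryItem is an inventory item actor that displays itself as a colored primitive shape with a score label.
; The construction script picks a sphere, cube, cylinder or cone mesh from InventoryData.Type and writes InventoryData.Score to the text render.
; It then creates a dynamic M_BaseColor instance tinted with a random ColorPallete entry, so color can change whenever construction reruns.
; The event graph has no active logic.
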(event EventBeginPlay)

(event Collision|EventActorBeginOverlap
  (params (OtherActor :type Actor%20Object%20Reference)))

(event EventTick
  (params (DeltaSeconds :type Float%20%28single-precision%29)))

(fn ConstructionScript
  (bind _inventorydata (Variables|Default|GetInventoryData))
  (Components|StaticMesh|SetStaticMesh (Variables|Default|GetStaticMesh) (Utilities|Select :Index (.type _inventorydata) :Sphere "/Engine/EngineMeshes/MaterialSphere.MaterialSphere" :Cube "/Engine/BasicShapes/Cube.Cube" :Cylinder "/Engine/BasicShapes/Cylinder.Cylinder" :Cone "/Engine/BasicShapes/Cone.Cone"))
  (Rendering|Components|TextRender|SetText (Variables|Default|GetTextRender) (Utilities|Text|ToText(Integer) (.score _inventorydata)))
  (bind _returnvalue (Rendering|Material|CreateDynamicMaterialInstance (Variables|Default|GetStaticMesh) 0 "/Game/Materials/M_BaseColor.M_BaseColor" "None" :!class /Script/Engine.PrimitiveComponent))
  (Rendering|Material|SetVectorParameterValue _returnvalue "Color" (.OutItem (Utilities|Array|Random (Variables|Default|GetColorPallete))) :!class /Script/Engine.MaterialInstanceDynamic))